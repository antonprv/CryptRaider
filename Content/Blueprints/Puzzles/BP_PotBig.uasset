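; BP_PotBig is a big pot puzzle prop that highlights through an overlay material on its static mesh.
; On BeginPlay it caps the overlay's draw distance and binds to the first-person pawn's grabber hit and not-hit events.
; OnOwnerHit applies the highlight material, while OnOwnerNotHit clears it after a short delay to reduce flickering.
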(event Custom|OnOwnerHit
  ;[0.15 0.15 0.15 0.5] Highlight
  (Rendering|Material|SetOverlayMaterial (Variables|Default|GetStaticMesh) (Variables|Default|GetHighlightMaterial) :!class /Script/Engine.MeshComponent))

(event Custom|OnOwnerNotHit
  ;[0.15 0.15 0.15 0.5] Delay to reduce flickering
  (Utilities|FlowControl|Delay (Variables|Default|GetHighlightStopDelay))
  (Rendering|Material|SetOverlayMaterial (Variables|Default|GetStaticMesh) 0 :!class /Script/Engine.MeshComponent))

(event EventBeginPlay
  (bind _returnvalue (Game|Player|GetPlayerPawn 0))
  (Rendering|Material|SetOverlayMaterialMaxDrawDistance (Variables|Default|GetStaticMesh) (Variables|Default|GetHighlight%20Draw%20Distance) :!class /Script/Engine.MeshComponent)
  (Class|KismetSystemLibrary|IsObjectOfSoftClass _returnvalue "/Game/Blueprints/Player/BP_FirstPersonPawn.BP_FirstPersonPawn_C"
    (:True
      (bind _asbp_first_person_pawn (Utilities|Casting|CastToBP_FirstPersonPawn _returnvalue))
      ;[0.15 0.15 0.15 0.5] Bind Events
      (EventDispatchers|BindEventtoOnGrabberHitObject _asbp_first_person_pawn (EventDispatchers|CreateEvent :!event Custom|OnOwnerHit))
      (EventDispatchers|BindEventtoOnGrabberNotHitObject _asbp_first_person_pawn (EventDispatchers|CreateEvent :!event Custom|OnOwnerNotHit)))))

(event Collision|EventActorBeginOverlap
  (params (OtherActor :type Actor%20Object%20Reference)))

(event EventTick
  (params (DeltaSeconds :type Float%20%28single-precision%29)))

(fn ConstructionScript)