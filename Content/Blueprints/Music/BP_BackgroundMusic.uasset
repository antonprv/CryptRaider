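; Background music manager that switches between main menu, game loop, safety (victory), secret, secret ending and alarm tracks through BackgroundMusic interface events.
; BeginPlay registers the audio components in the AllMusic set at a shared volume.
; Play events call StopAllBut, which stops the first other playing track, then PlayAfterDelay starts the chosen one, using EaseOutSpeed as start time, and calls EaseIn.
; StopAll stops every playing track.
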(event EventPlaySecretEnding
  (bind _cue_secretending (Variables|Default|GetCUE_SecretEnding))
  ;[0.15 0.15 0.15 0.5] BackgroundMusic interface
  (bind _allstopped (CallFunction|StopAllBut _cue_secretending))
  (if _allstopped
    (Utilities|PlayAfterDelay _cue_secretending)))

(event EventStopAll
  ;[0.15 0.15 0.15 0.5] BackgroundMusic interface
  (bind _valuepin (Utilities|Set|ForEachLoop(Set) (Variables|Default|GetAllMusic))
    (:then
      (if (Audio|Components|Audio|IsPlaying _valuepin)
        (Audio|Components|Audio|Stop _valuepin)))))

(event EventPlayAlarm
  (bind _cue_alarn (Variables|Default|GetCUE_Alarn))
  ;[0.15 0.15 0.15 0.5] BackgroundMusic interface
  (bind _allstopped (CallFunction|StopAllBut _cue_alarn))
  (if _allstopped
    (Utilities|PlayAfterDelay _cue_alarn)
    (if (Audio|Components|Audio|IsPlaying _cue_alarn)
      _)))

(event EventPlaySecret
  (bind _cue_secret (Variables|Default|GetCUE_Secret))
  ;[0.15 0.15 0.15 0.5] BackgroundMusic interface
  (bind _allstopped (CallFunction|StopAllBut _cue_secret))
  (if _allstopped
    (Utilities|PlayAfterDelay _cue_secret)))

(event EventPlayMainMenu
  ;[0.15 0.15 0.15 0.5] BackgroundMusic interface
  (bind _allstopped (CallFunction|StopAllBut))
  (if _allstopped
    (Utilities|PlayAfterDelay (Variables|Default|GetCUE_MainMenu))))

(event EventPlayGameLoop
  (bind _cue_gameloop (Variables|Default|GetCUE_GameLoop))
  ;[0.15 0.15 0.15 0.5] BackgroundMusic interface
  (bind _allstopped (CallFunction|StopAllBut _cue_gameloop))
  (if _allstopped
    (Utilities|PlayAfterDelay _cue_gameloop)))

(event EventPlayVictory
  (bind _cue_safety (Variables|Default|GetCUE_Safety))
  ;[0.15 0.15 0.15 0.5] BackgroundMusic interface
  (bind _allstopped (CallFunction|StopAllBut _cue_safety))
  (if _allstopped
    (Utilities|PlayAfterDelay _cue_safety)))

(event EventBeginPlay
  (bind _cue_mainmenu (Variables|Default|GetCUE_MainMenu))
  (bind _cue_secretending (Variables|Default|GetCUE_SecretEnding))
  (bind _cue_secret (Variables|Default|GetCUE_Secret))
  (bind _cue_alarn (Variables|Default|GetCUE_Alarn))
  (bind _cue_safety (Variables|Default|GetCUE_Safety))
  (bind _cue_gameloop (Variables|Default|GetCUE_GameLoop))
  ;[0.15 0.15 0.15 0.5] Form the track list
  (Utilities|FlowControl|Sequence
    (:then_0
      (Utilities|Set|Add (Variables|Default|GetAllMusic) _cue_mainmenu)
      (Audio|Components|Audio|SetVolumeMultiplier _cue_mainmenu (Variables|Default|GetMusicOverallVolume) :!class /Script/Engine.AudioComponent))
    (:then_1
      (Utilities|Set|Add (Variables|Default|GetAllMusic) _cue_safety)
      (Audio|Components|Audio|SetVolumeMultiplier _cue_safety (Variables|Default|GetMusicOverallVolume) :!class /Script/Engine.AudioComponent))
    (:then_2
      (Utilities|Set|Add (Variables|Default|GetAllMusic) _cue_gameloop)
      (Audio|Components|Audio|SetVolumeMultiplier _cue_gameloop (Variables|Default|GetMusicOverallVolume) :!class /Script/Engine.AudioComponent))
    (:then_3
      (Utilities|Set|Add (Variables|Default|GetAllMusic) _cue_secret)
      (Audio|Components|Audio|SetVolumeMultiplier _cue_secret (Variables|Default|GetMusicOverallVolume) :!class /Script/Engine.AudioComponent))
    (:then_4
      (Utilities|Set|Add (Variables|Default|GetAllMusic) _cue_secretending)
      (Audio|Components|Audio|SetVolumeMultiplier _cue_secretending (Variables|Default|GetMusicOverallVolume) :!class /Script/Engine.AudioComponent))
    (:then_5
      (Utilities|Set|Add (Variables|Default|GetAllMusic) _cue_alarn)
      (Audio|Components|Audio|SetVolumeMultiplier _cue_alarn (Variables|Default|GetMusicOverallVolume) :!class /Script/Engine.AudioComponent))))

(fn ConstructionScript)

(fn StopAllBut
  (params (SoundToRemain :type Audio%20Component%20Object%20Reference))
  (bind _valuepin (Utilities|Set|ForEachLoop(Set) (Variables|Default|GetAllMusic))
    (:then
      (if (!= _valuepin SoundToRemain)
        (if (Audio|Components|Audio|IsPlaying _valuepin)
          (Audio|Components|Audio|AdjustVolume _valuepin (Variables|Default|GetEaseOutSpeed) 0.0 "Linear" :!class /Script/Engine.AudioComponent)
          (Audio|Components|Audio|Stop _valuepin)
          (return true))))
    (:CompletedPin
      (return true))))