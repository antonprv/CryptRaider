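; Game mode for Crypt Raider that controls the start, pause, restart and quit flow of the game.
; It freezes time on BeginPlay, holding the game until StartGame is called.
; Game manager interface events pause and resume by setting global time dilation to zero or one, rather than using the engine's pause.
; RestartGame reopens the TestMap level, and QuitGame exits the application.
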(event EventBeginPlay
  ;[0.15 0.15 0.15 0.5] Stop time at game start
  (Utilities|Time|SetGlobalTimeDilation 0.0))

(event EventStartGame
  ;[0.15 0.15 0.15 0.5] IGame Manager Interfae
  (Utilities|Time|SetGlobalTimeDilation 1.0))

(event EventQuitGame
  ;[0.15 0.15 0.15 0.5] IGame Manager Interfae
  (Game|QuitGame 0 "Quit" false))

(event EventUnpauseGame
  ;[0.15 0.15 0.15 0.5] IGame Manager Interfae
  (Utilities|Time|SetGlobalTimeDilation 1.0))

(event EventPauseGame
  ;[0.15 0.15 0.15 0.5] IGame Manager Interfae
  (Utilities|Time|SetGlobalTimeDilation 0.0))

(event EventRestartGame
  ;[0.15 0.15 0.15 0.5] IGame Manager Interfae
  (Game|OpenLevel(byObjectReference) "/Game/Maps/TestMap.TestMap"))

(fn ConstructionScript)